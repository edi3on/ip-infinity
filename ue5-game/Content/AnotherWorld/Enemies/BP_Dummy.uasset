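; BP_Dummy is an enemy target dummy that takes damage from first-person projectiles and collapses when killed.
; While alive, a mesh hit by a BP_FirstPersonProjectile subtracts the projectile's damage from Health and destroys the projectile.
; When Health reaches zero or below, it marks itself dead and enables physics simulation on the mesh.
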(event `self.Mesh.OnComponentHit`
  (params (HitComponent :type "PrimitiveComponent Object Reference") (OtherActor :type "Actor Object Reference") (OtherComp :type "PrimitiveComponent Object Reference") (NormalImpulse :type "Vector Structure") (Hit :type "HitResult Structure (by ref)"))
  (if (`self.isAlive`)
    (bind _asbp_first_person_projectile (cast `/Game/FirstPerson/Blueprints/BP_FirstPersonProjectile` OtherActor))
    (bind _output_get (set `self.health` (- (`self.health`) (`/Game/FirstPerson/Blueprints/BP_FirstPersonProjectile.dmg` _asbp_first_person_projectile))))
    (`self.K2_DestroyActor` _asbp_first_person_projectile)
    (if (<= _output_get 0.0)
      (set `self.isAlive` false)
      (`PrimitiveComponent.SetSimulatePhysics` (`self.Mesh`) true))))

(fn `UserConstructionScript`)